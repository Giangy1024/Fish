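; Fish pawn that schools with nearby fish using boids flocking, or wanders to random points, inside its biom box.
; A looping Movement timer sphere-traces for neighbours, optionally limited to the same mesh or material, and blends weighted cohesion, separation and alignment into a steering direction.
; Tick applies that direction as movement input and eases rotation toward velocity.
; Leaving the box, lacking neighbours or hitting non-fish actors triggers a new random heading within the box.
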(event `self.ReceiveTick`
  (params (DeltaSeconds :type "Float (single-precision)"))
  (`|ExecutionSequence`
    (:`then_0`
      (`self.-Looking forward`)
      (`|ExecutionSequence`
        (:`then_0`
          (`/Engine/EditorBlueprintResources/StandardMacros.DoOnce` false
            (:`Completed`
              (`self.-FindNewLocationAndDirection`))))
        (:`then_1`
          _))
      (`self.AddMovementInput` (`self.Average_Acceleration`) (`self.Speed_Scale`))
      (if (`self._Escape_Biom`)
        (if (not (`self.Set Flock?`))
          (`self.-FindNewLocationAndDirection`)
          (set `self.Speed_Scale` (`KismetMathLibrary.RandomFloatInRange` 0.5 1.0)))
        (else
          (set `self.Speed_Scale` (`KismetMathLibrary.RandomFloatInRange` 0.7 1.0)))))
    (:`then_1`
      (if (<= (`KismetMathLibrary.VSize` (- (`self.Target_Location`) (`self.K2_GetActorLocation`))) 50.0)
        (bind _returnvalue (`KismetSystemLibrary.K2_SetTimer` null "Movement" 0.1 true))
        (set `self.Timer_Movement` _returnvalue)))
    (:`then_2`
      (if (and (`self._Escape_Biom`) (not (`KismetSystemLibrary.K2_IsValidTimerHandle` (`self.Timer_Movement`))))
        (bind _returnvalue_2 (`KismetSystemLibrary.K2_SetTimer` null "Movement" 0.1 true))
        (set `self.Timer_Movement` _returnvalue_2)))))

(event `self.ReceiveBeginPlay`
  (set `self.Alignment_Distance` (`self.Search_Radius`))
  (bind _returnvalue (`KismetSystemLibrary.K2_SetTimer` null "Movement" 0.1 true))
  (set `self.Timer_Movement` _returnvalue))

(event `self.CollisionComponent.OnComponentHit`
  (params (HitComponent :type "PrimitiveComponent Object Reference") (OtherActor :type "Actor Object Reference") (OtherComp :type "PrimitiveComponent Object Reference") (NormalImpulse :type "Vector Structure") (Hit :type "HitResult Structure (by ref)"))
  (cast `/StylizedSmallFishes/Blueprints/Details/BP_FishFlock` OtherActor
    (:`CastFailed`
      (`self.-FindNewLocationAndDirection`))))

(event `Movement`
  (bind _success (`self.-Sphere_Trace_For_Objects`))
  (if (and _success (`self.Set Flock?`))
    (`self.-Get_Neighbors_Info`)
    (`self.-Average_Normalize`)
    ;[1 1 1] Set World_Direction
    (set `self.Average_Acceleration` (+ (* (`self.Average_Location_Cohesion`) (`self.K_Cohesion`)) (* (`self.Average_Location_Separation`) (`self.K_Separation`)) (* (`self.Average_Velocity_Alignment`) (`self.K_Alignment`))))
    (if (`self._Escape_Biom`)
      (`self.-FindNewLocationAndDirection`))
    (else
      (`self.-FindNewLocationAndDirection`)
      (if (not (`self.Set Flock?`))
        (`KismetSystemLibrary.K2_ClearAndInvalidateTimerHandle` (`self.Timer_Movement`))))))

(fn `-Average_Normalize`
  (`|ExecutionSequence`
    (:`then_0`
      (if (!= (`self.Number_Neighbors_Cohesion`) 0)
        (set `self.Average_Location_Cohesion` (`KismetMathLibrary.Normal` (- (/ (`self.Average_Location_Cohesion`) (`self.Number_Neighbors_Cohesion`)) (`self.K2_GetActorLocation`))))
        (return)))
    (:`then_1`
      (if (!= (`self.Number_Neighbors_Separation`) 0)
        (set `self.Average_Location_Separation` (`KismetMathLibrary.Normal` (* (/ (`self.Average_Location_Separation`) (`self.Number_Neighbors_Separation`)) -1.0)))
        (return)))
    (:`then_2`
      (if (!= (`self.Number_Neighbors_Alignment`) 0)
        (set `self.Average_Velocity_Alignment` (`KismetMathLibrary.Normal` (/ (`self.Average_Velocity_Alignment`) (`self.Number_Neighbors_Alignment`))))
        (return)))))

(fn `-FindNewLocationAndDirection`
  (bind _box (`/Game/StylizedSmallFishes/Blueprints/BP_Fish_Flock.Box` (`self.Current_Biom`)))
  (bind _returnvalue (`KismetMathLibrary.RandomPointInBoundingBox` (`SceneComponent.K2_GetComponentLocation` _box) (`BoxComponent.BoxExtent` _box)))
  (set `self.Target_Location` _returnvalue)
  (set `self.Average_Acceleration` (`KismetMathLibrary.Normal` (- _returnvalue (`self.K2_GetActorLocation`))))
  (return))

(fn `-Get_Neighbors_Info`
  (set `self.Average_Location_Cohesion` (0.0 0.0 0.0))
  (set `self.Average_Location_Separation` (0.0 0.0 0.0))
  (set `self.Average_Velocity_Alignment` (0.0 0.0 0.0))
  (set `self.Number_Neighbors_Separation` 0)
  (set `self.Number_Neighbors_Cohesion` 0)
  (set `self.Number_Neighbors_Alignment` 0)
  (for _array_element (`self.Info`)
    (`|ExecutionSequence`
      (:`then_0`
        (bind (_actor _distance _location) (break `/Game/StylizedSmallFishes/Blueprints/Details/Str_Flock_Info` _array_element))
        (if (< _distance (`self.Cohesion_Distance`))
          (set `self.Average_Location_Cohesion` (+ (`self.Average_Location_Cohesion`) _location))
          (set `self.Number_Neighbors_Cohesion` (+ (`self.Number_Neighbors_Cohesion`) 1))))
      (:`then_1`
        (bind (_actor_2 _distance_2 _location_2) (break `/Game/StylizedSmallFishes/Blueprints/Details/Str_Flock_Info` _array_element))
        (if (< _distance_2 (`self.Separation_Distance`))
          (set `self.Average_Location_Separation` (+ (- _location_2 (`self.K2_GetActorLocation`)) (`self.Average_Location_Separation`)))
          (set `self.Number_Neighbors_Separation` (+ (`self.Number_Neighbors_Separation`) 1))))
      (:`then_2`
        (bind (_actor_3 _distance_3) (break `/Game/StylizedSmallFishes/Blueprints/Details/Str_Flock_Info` _array_element))
        (if (< _distance_3 (`self.Alignment_Distance`))
          (set `self.Average_Velocity_Alignment` (+ (`self.GetVelocity` _actor_3) (`self.Average_Velocity_Alignment`)))
          (set `self.Number_Neighbors_Alignment` (+ (`self.Number_Neighbors_Alignment`) 1))
          (if (and (== (`self.Number_Neighbors_Cohesion`) 0) (== (`self.Number_Neighbors_Separation`) 0) (> (`self.Number_Neighbors_Alignment`) 0))
            (set `self.Separation_Distance` (`self.Alignment_Distance`))))))))

(fn `-Looking forward`
  (`self.K2_SetActorRotation` (`|EaseFunction` "EaseInOut" 0.1 (`self.K2_GetActorRotation`) (`KismetMathLibrary.MakeRotFromX` (`KismetMathLibrary.Normal` (`self.GetVelocity`)))))
  (return))

(fn `-Sphere_Trace_For_Objects`
  (returns (Success :type Boolean))
  (bind _returnvalue (`self.K2_GetActorLocation`))
  (bind _fishtype (`self.FishType`))
  (`KismetArrayLibrary.Array_Clear` (`self.Info`))
  (`KismetArrayLibrary.Array_Clear` (`self.Neighbour`))
  (bind _outhits (`KismetSystemLibrary.SphereTraceMultiForObjects` _returnvalue _returnvalue (`self.Search_Radius`) (`|MakeArray` "ObjectTypeQuery3" :!type "EObjectTypeQuery Enum")))
  (for _array_element _outhits
    (bind _asbp_fish_flock (cast `/StylizedSmallFishes/Blueprints/Details/BP_FishFlock` (`.HitActor` (`GameplayStatics.BreakHitResult` _array_element))))
    (if (`self.RandomSpeciesInFlocks`)
      (`KismetArrayLibrary.Array_AddUnique` (`self.Neighbour`) _asbp_fish_flock :!label _label)
      (elif (== (select `/Game/StylizedSmallFishes/Blueprints/Details/e_FishType` _fishtype :`NewEnumerator0` (`StaticMeshComponent.StaticMesh` (`DefaultPawn.MeshComponent` _asbp_fish_flock)) :`NewEnumerator1` (`/StylizedSmallFishes/Blueprints/Details/BP_FishFlock.OriginMaterial` _asbp_fish_flock) :!type "Object Object Reference") (select `/Game/StylizedSmallFishes/Blueprints/Details/e_FishType` _fishtype :`NewEnumerator0` (`StaticMeshComponent.StaticMesh` (`self.MeshComponent`)) :`NewEnumerator1` (`self.OriginMaterial`) :!type "Object Object Reference"))
        (goto _label))))
  (for (_array_element_2 _array_index) (`self.Neighbour`)
    (bind _returnvalue_2 (`self.K2_GetActorLocation` _array_element_2))
    (`KismetArrayLibrary.Array_Set` (`self.Info`) _array_index (make `/Game/StylizedSmallFishes/Blueprints/Details/Str_Flock_Info` _array_element_2 (`KismetMathLibrary.VSize` (- (`self.K2_GetActorLocation`) _returnvalue_2)) _returnvalue_2) true))
  (if (> (`KismetArrayLibrary.Array_Length` (`self.Neighbour`)) 1)
    (return true)
    (else
      (return false))))

(fn `_Escape_Biom`
  (returns (Escape_Biom :type Boolean))
  (bind _box (`/Game/StylizedSmallFishes/Blueprints/BP_Fish_Flock.Box` (`self.Current_Biom`)))
  (bind _returnvalue (`SceneComponent.K2_GetComponentLocation` _box))
  (bind _boxextent (`BoxComponent.BoxExtent` _box))
  (return (`self.Check_Escape_Biom_Location` (+ _returnvalue _boxextent) (- _returnvalue _boxextent) (`self.K2_GetActorLocation`))))

(fn `UserConstructionScript`)